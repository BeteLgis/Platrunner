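; Game mode for a runner game that shows the run HUD and procedurally builds the floor track.
; BeginPlay lays an initial batch of tiles through AddFloorTile, which spawns a random straight piece at NextSpawnPoint.
; Each spawned tile's attach transform becomes the next spawn point, chaining the pieces end to end.
; A straight counter makes AddFloorTile insert a random corner after a fixed run of straights, then resets.
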(event `self.ReceiveBeginPlay`
  (bind _returnvalue (`|CreateWidget` "/Game/UMG/RunHUD.RunHUD_C"))
  (`UserWidget.AddToViewport` _returnvalue 0)
  (for _ (range 10)
    (`self.AddFloorTile`)))

(fn `AddFloorCorner`
  (bind _floorcorners (`self.FloorCorners`))
  (bind _returnvalue (`|SpawnActorFromClass` (`|GetArrayItem` _floorcorners (`KismetMathLibrary.RandomIntegerInRange` 0 (`KismetArrayLibrary.Array_LastIndex` _floorcorners))) (`self.NextSpawnPoint`) "Undefined" "OverrideRootScale" null null))
  (bind _asbp_floor_tile (cast `/Game/Blueprints/BP_FloorTile` _returnvalue))
  (bind _attachtransform (`/Game/Blueprints/BP_FloorTile.GetAttachTransform` _asbp_floor_tile))
  (set `self.NextSpawnPoint` _attachtransform)
  (set `self.CurrentStraights` 0))

(fn `AddFloorTile`
  (bind _floortiles (`self.FloorTiles`))
  (if (> (`self.CurrentStraights`) 7)
    (`self.AddFloorCorner`)
    (else
      (bind _returnvalue (`|SpawnActorFromClass` (`|GetArrayItem` _floortiles (`KismetMathLibrary.RandomIntegerInRange` 0 (`KismetArrayLibrary.Array_LastIndex` _floortiles))) (`self.NextSpawnPoint`) "Undefined" "OverrideRootScale" null null))
      (bind _asbp_floor_tile (cast `/Game/Blueprints/BP_FloorTile` _returnvalue))
      (bind _attachtransform (`/Game/Blueprints/BP_FloorTile.GetAttachTransform` _asbp_floor_tile))
      (set `self.NextSpawnPoint` _attachtransform)
      (set `self.CurrentStraights` (+ (`self.CurrentStraights`) 1)))))

(fn `UserConstructionScript`)