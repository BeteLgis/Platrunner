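; Obstacle actor that keeps moving its static mesh along the local Z axis.
; BeginPlay starts the first move with a random duration, then Move calls itself with a fixed duration to loop.
; Each move uses MoveComponentTo toward a target from GetNewTransform, which updates MoveDistance, adds it to the current relative Z, and keeps the rotation.
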(event `self.ReceiveBeginPlay`
  (`parent.ReceiveBeginPlay`)
  (`self.Move` (`KismetMathLibrary.RandomFloat`)))

(event `Move`
  (params (OverTime :type "Float (double-precision)" :default 1.0))
  (bind (_newlocation _newrotation) (`self.GetNewTransform`))
  (`KismetSystemLibrary.MoveComponentTo` (`self.StaticMesh`) _newlocation _newrotation false false OverTime)
  (`self.Move` 1.0))

(fn `GetNewTransform`
  (returns (NewLocation :type "Vector Structure") (NewRotation :type "Rotator Structure"))
  (bind _staticmesh (`self.StaticMesh`))
  (bind (_relativelocation_x _relativelocation_y _relativelocation_z) (`KismetMathLibrary.BreakVector` (`SceneComponent.RelativeLocation` _staticmesh)))
  (`/Engine/EditorBlueprintResources/StandardMacros.NegateFloat` (`self.MoveDistance`)
    (:`  `
      (return (`KismetMathLibrary.MakeVector` _relativelocation_x _relativelocation_y (+ _relativelocation_z (`self.MoveDistance`))) (`SceneComponent.RelativeRotation` _staticmesh)))))

(fn `UserConstructionScript`
  (`parent.UserConstructionScript`))