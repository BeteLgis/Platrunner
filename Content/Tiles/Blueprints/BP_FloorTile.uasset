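; BP_FloorTile is a three-lane floor segment for a runner game, exposing an attach transform and populating itself with obstacles and items.
; SpawnObstacles and SpawnItems add child actors at lane points or random box positions, weighted by the game mode's Difficulty.
; Its end trigger adds score, requests another tile from BP_RunGameMode, then destroys this one after a delay.
; Falling or re-crossing the entry trigger kills the runner.
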(event `self.EndTrigger.OnComponentBeginOverlap`
  (params (OverlappedComponent :type "PrimitiveComponent Object Reference") (OtherActor :type "Actor Object Reference") (OtherComp :type "PrimitiveComponent Object Reference") (OtherBodyIndex :type Integer) (bFromSweep :type Boolean) (SweepResult :type "HitResult Structure (by ref)"))
  ;[1 1 1] Add a new platform ahead and delete one behind
  (bind _asbp_run_character (cast `/Game/Character/Blueprints/BP_RunCharacter` OtherActor))
  (`/Game/Character/Blueprints/BP_RunCharacter.AddScore` _asbp_run_character)
  (bind _asbp_run_game_mode (cast `/Game/GameMode/BP_RunGameMode` (`GameplayStatics.GetGameMode`)))
  (`/Game/GameMode/BP_RunGameMode.AddFloorTile` _asbp_run_game_mode)
  (`KismetSystemLibrary.Delay` 2.0)
  (`self.K2_DestroyActor`))

(event `self.FallSpace.OnComponentBeginOverlap`
  (params (OverlappedComponent :type "PrimitiveComponent Object Reference") (OtherActor :type "Actor Object Reference") (OtherComp :type "PrimitiveComponent Object Reference") (OtherBodyIndex :type Integer) (bFromSweep :type Boolean) (SweepResult :type "HitResult Structure (by ref)"))
  ;[1 1 1] Fall of the platform or somehow glitched and running back
  (bind _asbp_run_character (cast `/Game/Character/Blueprints/BP_RunCharacter` OtherActor))
  (`/Game/Character/Blueprints/BP_RunCharacter.Death` _asbp_run_character false 0.0))

(event `self.EntryTrigger.OnComponentBeginOverlap`
  (params (OverlappedComponent :type "PrimitiveComponent Object Reference") (OtherActor :type "Actor Object Reference") (OtherComp :type "PrimitiveComponent Object Reference") (OtherBodyIndex :type Integer) (bFromSweep :type Boolean) (SweepResult :type "HitResult Structure (by ref)"))
  ;[1 1 1] Fall of the platform or somehow glitched and running back
  (bind _asbp_run_character (cast `/Game/Character/Blueprints/BP_RunCharacter` OtherActor))
  (if (`self.Entered`)
    (`/Game/Character/Blueprints/BP_RunCharacter.Death` _asbp_run_character false 0.0)
    (else
      (set `self.Entered` true))))

(fn `GetAttachTransform`
  (returns (AttachTransform :type "Transform Structure"))
  (return (`SceneComponent.K2_GetComponentToWorld` (`self.AttachPoint`))))

(fn `GetDifficulty`
  (returns (Difficulty :type "/Game/Lib/Difficulty Structure"))
  (bind _asbp_run_game_mode (cast `/Game/GameMode/BP_RunGameMode` (`GameplayStatics.GetGameMode`)))
  (return (`/Game/GameMode/BP_RunGameMode.Difficulty` _asbp_run_game_mode)))

(fn `Randomize`
  (params (Gaps :type "Array of Integer"))
  (returns (Lines :type "Array of Integer"))
  (bind _value (`/Game/Lib/Generator.GetRandom` Gaps))
  (bind _indexes (`/Game/Lib/Generator.SelectRandomIndexes` 2 (- 3 _value)))
  (return _indexes))

(fn `SetActiveLines`
  (set `self.ActiveLines` (`|MakeArray` true true true)))

(fn `SetSpawnAreas`
  (set `self.SpawnAreas` (`|MakeArray` (`self.ItemAreaL`) (`self.ItemAreaM`) (`self.ItemAreaR`))))

(fn `SetSpawnPoints`
  (set `self.SpawnPoints` (`|MakeArray` (`SceneComponent.GetRelativeTransform` (`self.SpawnPointL`)) (`SceneComponent.GetRelativeTransform` (`self.SpawnPointM`)) (`SceneComponent.GetRelativeTransform` (`self.SpawnPointR`)))))

(fn `SpawnItems`
  (locals (Line :type Integer :default 0))
  (bind _line (`local.Line`))
  (bind _output (`|GetArrayItem` (`self.SpawnAreas`) _line))
  (`self.SetSpawnAreas`)
  (bind _difficulty (`self.GetDifficulty`))
  (for _ (range (+ (`KismetMathLibrary.RandomIntegerInRange` 0 4) 1))
    (set `local.Line` (`KismetMathLibrary.RandomIntegerInRange` 0 2))
    (if (`|GetArrayItem` (`self.ActiveLines`) _line)
      (bind _value (`/Game/Lib/Generator.GetRandom` (`.Items_30_3E4DBD1D43D8B47731D748ACCA2177AD` (break `/Game/Lib/Difficulty` _difficulty))))
      (bind _returnvalue (`AddComponent|NODE_AddChildActorComponent-2` :`RelativeTransform` (`KismetMathLibrary.Conv_VectorToTransform` (`KismetMathLibrary.RandomPointInBoundingBox` (`SceneComponent.RelativeLocation` _output) (`BoxComponent.BoxExtent` _output)))))
      (`ChildActorComponent.SetChildActorClass` _returnvalue (`|GetArrayItem` (`self.Items`) _value)))))

(fn `SpawnObstacles`
  (`self.SetSpawnPoints`)
  (bind _difficulty (`self.GetDifficulty`))
  (bind (_tiles _gaps _obstacles) (break `/Game/Lib/Difficulty` _difficulty))
  (bind _lines (`self.Randomize` _gaps))
  (for _array_element _lines
    (if (`|GetArrayItem` (`self.ActiveLines`) _array_element)
      (bind _value (`/Game/Lib/Generator.GetRandom` _obstacles))
      (bind _returnvalue (`AddComponent|NODE_AddChildActorComponent-3` :`RelativeTransform` (`|GetArrayItem` (`self.SpawnPoints`) _array_element)))
      (`ChildActorComponent.SetChildActorClass` _returnvalue (`|GetArrayItem` (`self.Obstacles`) _value)))))

(fn `UserConstructionScript`
  (`self.SetActiveLines`))