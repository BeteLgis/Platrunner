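; BP_FloorTile_Gap is a floor tile variant that opens gaps across its three floor lines.
; The construction script gathers the three floor components into an array, then runs the parent script.
; SetActiveLines passes the difficulty's Gaps value to Randomize to pick gap indices, recording each line as active or not.
; Picked floors are hidden with their children and lose collision; the event graph is empty.
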(fn `SetActiveLines`
  (bind _difficulty (`self.GetDifficulty`))
  (bind _lines (`self.Randomize` (`.Gaps_21_1BE5840D4A5B2AD21405E288348493A1` (break `/Game/Lib/Difficulty` _difficulty))))
  (for _index (range 3)
    (bind _returnvalue (`KismetArrayLibrary.Array_Contains` _lines _index))
    (`KismetArrayLibrary.Array_Add` (`self.ActiveLines`) (not _returnvalue))
    (if _returnvalue
      (bind _output (`|GetArrayItem` (`self.Floors`) _index))
      (`SceneComponent.SetVisibility` _output false true)
      (`PrimitiveComponent.SetCollisionEnabled` _output "NoCollision"))))

(fn `UserConstructionScript`
  (set `self.Floors` (`|MakeArray` (`self.Floor0`) (`self.Floor1`) (`self.Floor2`)))
  (`parent.UserConstructionScript`))